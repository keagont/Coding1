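; BP_Item is an item actor with a name, damage value and elemental type, which prints a greeting with its name on BeginPlay.
; The construction script replaces the default "Item" name with a random pick from a hardcoded list, whose upper index is one past the end.
; GetDamage doubles damage when its element sits two steps from the other element in a four-type cycle, otherwise returning base damage.
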(event EventBeginPlay
  (Development|PrintString (Utilities|String|Append "Hello, my name is " (Variables|Default|GetName))))

(event Collision|EventActorBeginOverlap
  (params (OtherActor :type Actor%20Object%20Reference)))

(event EventTick
  (params (DeltaSeconds :type Float%20%28single-precision%29)))

(fn ConstructionScript
  (bind _returnvalue (Utilities|String|MakeLiteralString "Dave"))
  (bind _returnvalue_2 (Utilities|String|MakeLiteralString "Joe"))
  (bind _returnvalue_3 (Utilities|String|MakeLiteralString "Dale"))
  (bind _returnvalue_4 (Utilities|String|MakeLiteralString "Daniel"))
  (bind _returnvalue_5 (Utilities|String|MakeLiteralString "Alex"))
  (bind _returnvalue_6 (Utilities|String|MakeLiteralString "Greg"))
  (bind _array (Utilities|Array|MakeArray _returnvalue_2 _returnvalue_3 _returnvalue_4 _returnvalue_5 _returnvalue_6 _returnvalue))
  (if (Utilities|Enum|Equal(Enum) (Variables|Default|GetName) "Item")
    (Variables|Default|SetName (Utilities|Array|Get(acopy) _array (Math|Random|RandomIntegerinRange 0 (Utilities|Array|Length _array))))))

(fn GetDamage
  (params (OtherElementalType :type Enum_ElementalType%20Enum :default "NewEnumerator1"))
  (if (== (Variables|Default|GetElementalType) (Class|KismetMathLibrary|PercentByteByte (+ OtherElementalType 2) 4))
    (LocalVariables|SetReturnedDamage (* (Variables|Default|GetDamage) 2))
    (else
      (LocalVariables|SetReturnedDamage (Variables|Default|GetDamage))))
  (return (LocalVariables|GetReturnedDamage)))