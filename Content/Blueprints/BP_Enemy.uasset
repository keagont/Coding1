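; BP_Enemy is an enemy actor that dies when the third-person player character overlaps its capsule.
; On BeginPlay it takes a random name from a shuffled list and, unless a team material is already set, picks one at random for its meshes.
; The overlap drops Health below zero, and a repeating Delay loop polls Health, printing a kill message with the name before destroying the actor.
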(event OnComponentBeginOverlap(Capsule)
  (params (OverlappedComponent :type Primitive%20Component%20Object%20Reference) (OtherActor :type Actor%20Object%20Reference) (OtherComp :type Primitive%20Component%20Object%20Reference) (OtherBodyIndex :type Integer) (bFromSweep :type Boolean) (SweepResult :type Hit%20Result%20Structure%20%28by%20ref%29))
  (Utilities|Casting|CastToBP_ThirdPersonCharacter OtherActor)
  (Variables|Default|SetHealth -1.0))

(event EventBeginPlay
  (bind _names (Variables|Default|GetNames))
  (bind _materials (Variables|Default|GetMaterials))
  (Utilities|FlowControl|Sequence
    (:then_0
      (Utilities|FlowControl|Delay 0.2 :!label _label)
      (if (<= (Variables|Default|GetHealth) 0.0)
        (Development|PrintString (Utilities|String|Append "You Killed " (Utilities|String|ToString(Name) (Variables|Default|GetEnemyName))))
        (Actor|DestroyActor)
        (else
          (goto _label))))
    (:then_1
      (Utilities|Array|Shuffle _names)
      (Variables|Default|SetEnemyName (Utilities|Array|Get(acopy) _names)))
    (:then_2
      (Utilities|IsValid (Variables|Default|GetEnemyTeamMaterial)
        (:Is%20Valid
          _)
        (:Is%20Not%20Valid
          (Utilities|Array|Shuffle _materials)
          (Variables|Default|SetEnemyTeamMaterial (Utilities|Array|Get(acopy) _materials))))
      (Rendering|Material|SetMaterial (Variables|Default|GetBody) 0 (Variables|Default|GetEnemyTeamMaterial)))))

(fn ConstructionScript)

(fn DetectLocation)