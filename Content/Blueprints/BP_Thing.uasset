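; BP_Thing is a demo of Blueprint functions that prints messages to the screen on BeginPlay.
; A custom Say event prints text in random colors, used for a greeting and by CountToNumber, which counts with increasing display durations.
; It then prints each entry in Names, colored by GetColorByNameLength: black for short names, shading through magenta for medium ones, and white for long ones.
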(event Custom|Say
  (params (InString :type String) (Duration :type Float%20%28single-precision%29))
  (bind _returnvalue (Math|Random|RandomUnitVector))
  (Development|PrintString InString true true (Utilities|Struct|MakeLinearColor (.x _returnvalue) (.y _returnvalue) (.z _returnvalue) 1.0) Duration))

(event EventBeginPlay
  (bind _names (Variables|Default|GetNames))
  (Development|PrintString "Welcome to Functions")
  (CallFunction|Say "Hello" 5.0)
  (CallFunction|CounttoNumber 10)
  (for _index (range 0 (Utilities|Array|Length _names))
    (bind _output (CallFunction|GetColorbyNameLength (Utilities|Array|Get(acopy) _names _index)))
    (Development|PrintString (Utilities|Array|Get(acopy) _names _index) true true _output 6.0)))

(fn ConstructionScript)

(fn CounttoNumber
  (params (Number :type Integer))
  (for _index (range 0 Number)
    (CallFunction|Say (Utilities|String|ToString(Integer) _index) (+ (* _index 0.1) 5.0)))
  (return))

(fn GetColorbyNameLength
  (params (Input :type String))
  (bind _returnvalue (Utilities|String|Len Input))
  (bind _returnvalue_2 (- _returnvalue 5))
  (bind _returnvalue_3 (* _returnvalue_2 0.2))
  (if (<= _returnvalue 5)
    (Variables|Default|SetOutputColor (Utilities|Struct|MakeLinearColor 0.0 0.0 0.0 1.0))
    (elif (>= _returnvalue 10)
      (Variables|Default|SetOutputColor "(R=1.000000,G=1.000000,B=1.000000,A=1.000000)")
      (else
        (Variables|Default|SetOutputColor (Utilities|Struct|MakeLinearColor _returnvalue_3 0.0 _returnvalue_3 1.0)))))
  (return (Variables|Default|GetOutputColor)))