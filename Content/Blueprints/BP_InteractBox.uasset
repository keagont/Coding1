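; BP_InteractBox is an interactable actor that opens a test shop menu.
; On BeginPlay it creates and caches a W_TestShop widget.
; Its Interact event adds that widget to the viewport, switches the player to UI-only input with the cursor shown, and pauses the game.
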(event EventBeginPlay
  (bind _returnvalue (UserInterface|CreateWidget "/Game/Widgets/W_TestShop.W_TestShop_C"))
  (Variables|Default|SetW_TestShop _returnvalue))

(event Collision|EventActorBeginOverlap
  (params (OtherActor :type Actor%20Object%20Reference)))

(event EventTick
  (params (DeltaSeconds :type Float%20%28single-precision%29)))

(event EventInteract
  (bind _returnvalue (Game|GetPlayerController 0))
  (bind _w_testshop (Variables|Default|GetW_TestShop))
  (UserInterface|Viewport|AddtoViewport _w_testshop 0)
  (Input|SetInputModeUIOnly _returnvalue _w_testshop "DoNotLock" false)
  (Variables|/Script/Engine.PlayerController|SetbShowMouseCursor _returnvalue true)
  (Game|SetGamePaused true))

(fn ConstructionScript)