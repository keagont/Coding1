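; BP_GreenKey is a green key pickup that adds to the player's key count.
; When its Sphere component registers a hit from BP_ThirdPersonCharacter, it increments that character's GreenKeys, prints the new total and destroys itself.
; Collection relies on a blocking hit rather than an overlap, and BeginPlay prints a debug message confirming the key exists.
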(event OnComponentHit(Sphere)
  (params (HitComponent :type Primitive%20Component%20Object%20Reference) (OtherActor :type Actor%20Object%20Reference) (OtherComp :type Primitive%20Component%20Object%20Reference) (NormalImpulse :type Vector :default "0, 0, 0") (Hit :type Hit%20Result%20Structure%20%28by%20ref%29))
  (bind _asbp_third_person_character (Utilities|Casting|CastToBP_ThirdPersonCharacter OtherActor))
  (bind _result (Math|Integer|IncrementInt (Variables|/Game/ThirdPerson/Blueprints/BP_ThirdPersonCharacter.BP_ThirdPersonCharacter_C|GetGreenKeys _asbp_third_person_character))
    (:%20%20
      (bind _output_get (Variables|/Game/ThirdPerson/Blueprints/BP_ThirdPersonCharacter.BP_ThirdPersonCharacter_C|SetGreenKeys _asbp_third_person_character _result))
      (Development|PrintString (Utilities|String|Append "Loot Get! Green Keys: " (Utilities|String|ToString(Integer) _output_get)))
      (Actor|DestroyActor))))

(event EventBeginPlay
  (Development|PrintString (Utilities|String|Append (Utilities|GetDisplayName "BP_GreenKey") " exists")))

(event Collision|EventActorBeginOverlap
  (params (OtherActor :type Actor%20Object%20Reference)))

(event EventTick
  (params (DeltaSeconds :type Float%20%28single-precision%29)))

(fn ConstructionScript)