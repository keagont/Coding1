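; Enemy spawner that keeps the level populated by refilling it with BP_Enemy once none remain.
; On BeginPlay it gathers and counts all BP_EnemySpawnLocation actors, then spawns enemies at their transforms, each location passing a random roll of roughly 80%.
; A self-calling check polls the live enemy count every two seconds and triggers a new wave when it reaches zero.
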(event Custom|SpawnEnemy
  ;[1 1 1] Spawn Enemies
  (for _array_element (stale EventBeginPlay _outactors)
    (if (> (Math|Random|RandomFloat) 0.2)
      (Game|SpawnActorfromClass "/Game/Blueprints/BP_Enemy.BP_Enemy_C" (Transformation|GetActorTransform _array_element) "Undefined" "MultiplyWithRoot" 0 0))))

(event Custom|Enemy%20Count%20Check
  ;[1 1 1] Check amount of enemies
  (bind _outactors (Actor|GetAllActorsOfClass "/Game/Blueprints/BP_Enemy.BP_Enemy_C"))
  (if (> (Utilities|Array|Length _outactors) 0)
    (Utilities|FlowControl|Delay 2.0)
    (else
      (CallFunction|SpawnEnemy)))
  (CallFunction|EnemyCountCheck))

(event EventBeginPlay
  ;[1 1 1] Set up enemies
  (bind _outactors (Actor|GetAllActorsOfClass "/Game/Blueprints/BP_EnemySpawnLocation.BP_EnemySpawnLocation_C"))
  (Development|PrintString (Utilities|String|Append "There are " (Utilities|String|ToString(Integer) (Utilities|Array|Length _outactors)) " Spawners in the world"))
  (CallFunction|SpawnEnemy)
  (CallFunction|EnemyCountCheck))

(fn ConstructionScript)