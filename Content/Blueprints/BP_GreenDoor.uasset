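; BP_GreenDoor is a locked door that the player opens by bumping into it while holding a green key.
; A hit on its Cube component casts the other actor to BP_ThirdPersonCharacter and checks its GreenKeys count.
; With a key it decrements the count, prints the remaining total and destroys the door; otherwise it prints a no-key message.
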(event OnComponentHit(Cube)
  (params (HitComponent :type Primitive%20Component%20Object%20Reference) (OtherActor :type Actor%20Object%20Reference) (OtherComp :type Primitive%20Component%20Object%20Reference) (NormalImpulse :type Vector :default "0, 0, 0") (Hit :type Hit%20Result%20Structure%20%28by%20ref%29))
  (bind _asbp_third_person_character (Utilities|Casting|CastToBP_ThirdPersonCharacter OtherActor))
  (if (> (Variables|/Game/ThirdPerson/Blueprints/BP_ThirdPersonCharacter.BP_ThirdPersonCharacter_C|GetGreenKeys _asbp_third_person_character) 0)
    (Development|PrintString "Unlocked")
    (bind _output_get (Variables|/Game/ThirdPerson/Blueprints/BP_ThirdPersonCharacter.BP_ThirdPersonCharacter_C|SetGreenKeys _asbp_third_person_character (- (Variables|/Game/ThirdPerson/Blueprints/BP_ThirdPersonCharacter.BP_ThirdPersonCharacter_C|GetGreenKeys _asbp_third_person_character) 1)))
    (Development|PrintString (Utilities|String|Append "Green Keys: " (Utilities|String|ToString(Integer) _output_get)))
    (Actor|DestroyActor)
    (else
      (Development|PrintString "NO KEY!"))))

(event EventBeginPlay)

(event Collision|EventActorBeginOverlap
  (params (OtherActor :type Actor%20Object%20Reference)))

(event EventTick
  (params (DeltaSeconds :type Float%20%28single-precision%29)))

(fn ConstructionScript)