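; BP_CoolBox is an actor with a Cube component that spawns BP_Key actors above itself.
; BeginPlay caches a spawn point 200 units above the Cube's world location and prints both positions for debugging.
; Tick spawns a new BP_Key at that cached point every frame, with no limit or condition.
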(event EventBeginPlay
  (bind _cube (Variables|Default|GetCube))
  (bind _returnvalue (Transformation|GetWorldLocation _cube))
  (bind _output_get (Variables|Default|SetKeySpawnLocation (+ _returnvalue "0.000000,0.000000,200.000000")))
  (Development|PrintString (Utilities|String|ToString(Vector) _returnvalue) true true "(R=0.000000,G=0.660000,B=1.000000,A=1.000000)" 1e+01)
  (Development|PrintString (Utilities|String|ToString(Vector) _output_get) true true "(R=0.000000,G=0.660000,B=1.000000,A=1.000000)" 1e+01))

(event Collision|EventActorBeginOverlap
  (params (OtherActor :type Actor%20Object%20Reference)))

(event EventTick
  (params (DeltaSeconds :type Float%20%28single-precision%29))
  (Game|SpawnActorfromClass "/Game/Blueprints/BP_Key.BP_Key_C" (Math|Transform|MakeTransform (stale EventBeginPlay _output_get) "0, 0, 0" "1.000000,1.000000,1.000000") "Undefined" "MultiplyWithRoot" 0 0))

(fn ConstructionScript)